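; Cannon actor that automatically and repeatedly fires EnemyBullet_BP projectiles for as long as it is in play.
; From BeginPlay it waits FireRate, spawns a bullet at ProjectileSpawnPoint's transform scaled by ProjectileScale, then plays CannonFireTimeline.
; The timeline slides the barrel along its local Y axis, and its Cannon Fire event track loops back to the delay for the next shot.
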(event `self.ReceiveBeginPlay`
  (`KismetSystemLibrary.Delay` (`self.Fire Rate`) :!label _label)
  (`self.Spawn Projectile`)
  (bind (_direction _cannon_barrel_location) (`Timeline|Cannon Fire Timeline` :!via `PlayFromStart`)
    (:`Update`
      (`self.Move Cannon Barrel` _cannon_barrel_location))
    (:`Cannon Fire`
      (goto _label))))

(fn `Move Cannon Barrel`
  (params (Alpha :type "Float (double-precision)"))
  (`SceneComponent.K2_SetRelativeLocation` (`self.CannonBarrel`) (`KismetMathLibrary.MakeVector` 0.0 (* Alpha 25.0)) false false))

(fn `Spawn Projectile`
  (bind _projectile_spawn_point (`self.Projectile Spawn Point`))
  (`|SpawnActorFromClass` "/Game/MyContent/Blueprints/Actors/Projectile/EnemyBullet_BP.EnemyBullet_BP_C" (`KismetMathLibrary.MakeTransform` (`SceneComponent.K2_GetComponentLocation` _projectile_spawn_point) (`SceneComponent.K2_GetComponentRotation` _projectile_spawn_point) (`KismetMathLibrary.Conv_DoubleToVector` (`self.Projectile Scale`))) "Undefined" "OverrideRootScale" null null))

(fn `UserConstructionScript`)