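; AmmoCollectable_BP is a collectable pickup that gives ammo to a Marine.
; On overlap with a Marine_BP it stores the Marine and passes to the parent's overlap handling only if that Marine's ammo is not full.
; It binds to the parent's OnCollected event at BeginPlay, and on collection adds AmmoPickupAmount to the stored Marine.
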(event `self.ReceiveBeginPlay`
  (add `self.On Collected` (delegate `On Execute`)))

(event `On Execute`
  (`/Game/MyContent/Blueprints/Pawns/Marine_BP.Add Ammo` (`self.Marine`) (`self.Ammo Pickup Amount`)))

(event `self.ReceiveActorBeginOverlap`
  (params (OtherActor :type "Actor Object Reference"))
  (bind _asmarine_bp (cast `/Game/MyContent/Blueprints/Pawns/Marine_BP` OtherActor))
  (bind _output_get (set `self.Marine` _asmarine_bp))
  (if (not (`/Game/MyContent/Blueprints/Pawns/Marine_BP.Is Ammo Full` _output_get))
    (`parent.ReceiveActorBeginOverlap` (`self.Marine`))))

(fn `UserConstructionScript`
  (`parent.UserConstructionScript`))