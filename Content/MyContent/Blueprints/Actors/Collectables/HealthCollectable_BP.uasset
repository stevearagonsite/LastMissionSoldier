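; HealthCollectable_BP is a health pickup that restores a set amount of health to the Marine.
; On overlap it stores the Marine and runs the parent overlap logic only when that Marine's health is not full, so full-health players do not trigger it.
; Healing is bound at BeginPlay to the inherited OnCollected event, which adds the health and prints a red debug message.
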(event `self.ReceiveBeginPlay`
  (add `self.On Collected` (delegate `On Execute`)))

(event `On Execute`
  (`/Game/MyContent/Blueprints/Pawns/Marine_BP.Add Health` (`self.Marine`) (`self.Health Pickup Amount`))
  (`KismetSystemLibrary.PrintString` "Health" true true (struct :`R` 1.0 :`A` 1.0)))

(event `self.ReceiveActorBeginOverlap`
  (params (OtherActor :type "Actor Object Reference"))
  (bind _asmarine_bp (cast `/Game/MyContent/Blueprints/Pawns/Marine_BP` OtherActor))
  (bind _output_get (set `self.Marine` _asmarine_bp))
  (if (not (`/Game/MyContent/Blueprints/Pawns/Marine_BP.Is Health Full` _output_get))
    (`parent.ReceiveActorBeginOverlap` (`self.Marine`))))

(fn `UserConstructionScript`
  (`parent.UserConstructionScript`))