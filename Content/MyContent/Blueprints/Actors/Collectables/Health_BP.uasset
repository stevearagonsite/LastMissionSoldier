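; Health collectable actor that plays a pickup animation when the player overlaps it, then destroys itself; no health change is applied here.
; On overlap it stores its starting location, scale and light intensity, then plays CollectionTimeline.
; Timeline curves lerp it toward the player's live location, shrink it to zero scale and drive the PointLight intensity directly, leaving the stored intensity unused.
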(event `self.ReceiveTick`
  (params (DeltaSeconds :type "Float (single-precision)")))

(event `self.ReceiveActorBeginOverlap`
  (params (OtherActor :type "Actor Object Reference"))
  (`/Game/MyContent/Blueprints/Libraries/MacroLibrary.IsPlayer` OtherActor
    (:`IsPlayer`
      (`self.Store Starting Values`)
      (bind (_direction _actor_location_alpha _actor_scale_alpha _actor_light_intensity_alpha) (`Timeline|Collection Timeline`)
        (:`Update`
          (`self.Move To Player` _actor_location_alpha)
          (`self.Object To Scale 0` _actor_scale_alpha)
          (`self.Changes Intensity 0` _actor_light_intensity_alpha))
        (:`Finished`
          (`self.K2_DestroyActor`))))))

(fn `Changes Intensity 0`
  (params (Alpha :type "Float (double-precision)"))
  (`LightComponent.SetIntensity` (`self.PointLight`) Alpha))

(fn `Move To Player`
  (params (Alpha :type "Float (double-precision)"))
  (`self.K2_SetActorLocation` (`KismetMathLibrary.VLerp` (`self.Start Location`) (`self.K2_GetActorLocation` (`GameplayStatics.GetPlayerCharacter` 0)) Alpha)))

(fn `Object To Scale 0`
  (params (Alpha :type "Float (double-precision)"))
  (`self.SetActorScale3D` (`KismetMathLibrary.VLerp` (`self.Start Scale`) (0.0 0.0 0.0) Alpha)))

(fn `Store Starting Values`
  (set `self.Start Location` (`self.K2_GetActorLocation`))
  (set `self.Start Scale` (`self.GetActorScale3D`))
  (set `self.Start Light Intensity` (`LightComponentBase.Intensity` (`self.PointLight`))))

(fn `UserConstructionScript`)