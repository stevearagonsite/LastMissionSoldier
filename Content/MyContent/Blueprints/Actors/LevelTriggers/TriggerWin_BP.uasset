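; TriggerWin_BP is a level trigger that completes the current level when the player overlaps it.
; After a one-second delay it opens the next entry in LevelNames, found from the current level's name, or quits the game on the last one.
; The crystal check counts CrystalCollectable_BP actors with >= 0, so it always passes; a win screen and movement lock remain a TODO.
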(event `self.ReceiveActorBeginOverlap`
  (params (OtherActor :type "Actor Object Reference"))
  (`/Game/MyContent/Blueprints/Libraries/MacroLibrary.IsPlayer` OtherActor
    (:`IsPlayer`
      (if (`self.Any Crystals Remaining`)
        ;[1 1 1] TODO: Screen Win and disable player movement
        (`KismetSystemLibrary.Delay` 1.0)
        (`self.Complete Level`)))))

(fn `Any Crystals Remaining`
  (returns (ReturnValue :type Boolean))
  (bind _outactors (`GameplayStatics.GetAllActorsOfClass` "/Game/MyContent/Blueprints/Actors/Collectables/CrystalCollectable_BP.CrystalCollectable_BP_C"))
  (return (>= (`KismetArrayLibrary.Array_Length` _outactors) 0)))

(fn `Complete Level`
  (if (`self.Is Final Level`)
    (`KismetSystemLibrary.QuitGame` null "Quit")
    (else
      (`self.Load Next Level`))))

(fn `Get Current Level Index`
  (returns (Index :type Integer))
  (bind _returnvalue (`GameplayStatics.GetCurrentLevelName` true))
  (return (`KismetArrayLibrary.Array_Find` (`self.Level names`) (`KismetStringLibrary.Conv_StringToName` _returnvalue))))

(fn `Get Next Level Name`
  (returns (Output :type "Name (by ref)"))
  (return (`|GetArrayItem` (`self.Level names`) (+ (`self.Get Current Level Index`) 1))))

(fn `Is Final Level`
  (returns (ReturnValue :type Boolean))
  (return (== (`KismetArrayLibrary.Array_LastIndex` (`self.Level names`)) (`self.Get Current Level Index`))))

(fn `Load Next Level`
  (`GameplayStatics.OpenLevel` (`self.Get Next Level Name`)))

(fn `UserConstructionScript`)