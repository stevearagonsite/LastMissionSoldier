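; Player marine pawn for what appears to be a twin-stick shooter, with world-axis movement, jumping, health and ammo.
; Tick turns control rotation from smoothed mouse velocity or thumbstick direction, past deadzones, switching on the last pressed key's device.
; Held fire loops projectile spawns at FireRate, gated by CanJump rather than ammo.
; Damage lowers health, sets Dead at zero, then unconditionally stops firing, calls death and triggers a one-time fade and level reload.
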(event `self.ReceiveTick`
  (params (DeltaSeconds :type "Float (single-precision)"))
  (`self.Update Player Aim`))

(event `Key|AnyKey`
  (params (Key :type "Key Structure"))
  (:`Pressed`
    (set `self.Gamepad Active` (`KismetInputLibrary.Key_IsGamepadKey` Key))))

(event `InputAxis|MoveForward`
  (params (AxisValue :type "Float (single-precision)"))
  (if (`self.Is Alive`)
    (`self.AddMovementInput` (1.0 0.0 0.0) AxisValue)))

(event `InputAxis|MoveRight`
  (params (AxisValue :type "Float (single-precision)"))
  (if (`self.Is Alive`)
    (`self.AddMovementInput` (0.0 1.0 0.0) AxisValue)))

(event `InputAction|Jump`
  (params (Key :type "Key Structure"))
  (:`Pressed`
    (if (`self.Is Alive`)
      (`self.Jump`))))

(event `InputAction|FireWeapon`
  (params (Key :type "Key Structure"))
  (:`Pressed`
    (set `self.IsFiring` true)
    (`self.Update Fire` :!label _label))
  (:`Released`
    (set `self.IsFiring` false)
    (goto _label)))

(event `self.ReceiveAnyDamage`
  (params (Damage :type "Float (single-precision)") (DamageType :type "DamageType Object Reference") (InstigatedBy :type "Controller Object Reference") (DamageCauser :type "Actor Object Reference"))
  (bind _health (`self.Decrease Health` Damage))
  (set `self.Dead` (<= _health 0.0))
  (set `self.IsFiring` false)
  (`self.OnDeath`)
  (`self.PlayerLost`))

(fn `Add Ammo`
  (params (`Add Ammo` :type "Float (double-precision)"))
  (set `self.Ammo` (`KismetMathLibrary.FClamp` (+ (`self.Ammo`) `Add Ammo`) 0.0 (`self.Max Ammo`))))

(fn `Add Health`
  (params (`Health To Add` :type "Float (double-precision)"))
  (set `self.Health` (`KismetMathLibrary.FClamp` (+ (`self.Health`) `Health To Add`) 0.0 100.0)))

(fn `Can Fire`
  (returns (ReturnValue :type Boolean))
  (return (`self.CanJump`)))

(fn `Decrease Health`
  (params (`Damage Amount` :type "Float (double-precision)"))
  (returns (Health :type "Float (double-precision)"))
  (bind _output_get (set `self.Health` (`KismetMathLibrary.FClamp` (- (`self.Health`) `Damage Amount`) 0.0 100.0)))
  (return _output_get))

(fn `Get Mouse Aim Direction`
  (returns (ReturnValue :type "Rotator Structure"))
  (bind (_returnvalue_x _returnvalue_y) (`KismetMathLibrary.BreakVector2D` (`self.Get Mouse Velocity`)))
  (return (`KismetMathLibrary.RInterpTo` (`Controller.GetControlRotation` (`GameplayStatics.GetPlayerController` 0)) (`KismetMathLibrary.MakeRotator` 0.0 0.0 (`KismetMathLibrary.DegAtan2` _returnvalue_x _returnvalue_y)) (`GameplayStatics.GetWorldDeltaSeconds`) (`self.Mouse Smoothing Strength`))))

(fn `Get Mouse Velocity`
  (returns (ReturnValue :type "Vector2D Structure"))
  (bind (_deltax _deltay) (`PlayerController.GetInputMouseDelta` (`GameplayStatics.GetPlayerController` 0)))
  (return (/ (`KismetMathLibrary.MakeVector2D` _deltax _deltay) (`GameplayStatics.GetWorldDeltaSeconds`))))

(fn `Get Thumbstick Aim Direction`
  (returns (ReturnValue :type "Rotator Structure"))
  (return (`KismetMathLibrary.MakeRotator` 0.0 0.0 (`KismetMathLibrary.DegAtan2` (`self.GetInputAxisValue`) (`self.GetInputAxisValue`)))))

(fn `Is Alive`
  (returns (ReturnValue :type Boolean))
  (return (not (`self.Dead`))))

(fn `Is Ammo Full`
  (returns (ReturnValue :type Boolean))
  (return (>= (`self.Ammo`) (`self.Max Ammo`))))

(fn `Is Health Full`
  (returns (ReturnValue :type Boolean))
  (return (>= (`self.Health`) 100.0)))

(fn `Is Mouse Above Deadzone`
  (returns (ReturnValue :type Boolean))
  (bind (_returnvalue_x _returnvalue_y) (`KismetMathLibrary.BreakVector2D` (`self.Get Mouse Velocity`)))
  (return (> (`KismetMathLibrary.VSize2D` (`KismetMathLibrary.MakeVector2D` _returnvalue_x _returnvalue_y)) (`self.Mouse Deadzone`))))

(fn `Is Thumbstick Above Deadzone`
  (returns (ReturnValue :type Boolean))
  (return (> (`KismetMathLibrary.VSize2D` (`KismetMathLibrary.MakeVector2D` (`self.GetInputAxisValue`) (`self.GetInputAxisValue`))) (`self.Thumbstick Deadzone`))))

(fn `Spawn Projectile`
  (bind _projectile_spawn_point (`self.Projectile Spawn Point`))
  (set `self.Ammo` (- (`self.Ammo`) 1.0))
  (`|SpawnActorFromClass` "/Game/MyContent/Blueprints/Actors/Projectile/HeroBullet_BP.HeroBullet_BP_C" (`KismetMathLibrary.MakeTransform` (`SceneComponent.K2_GetComponentLocation` _projectile_spawn_point) (`SceneComponent.K2_GetComponentRotation` _projectile_spawn_point) (`KismetMathLibrary.Conv_DoubleToVector` (`self.Projectile Scale`))) "Undefined" "OverrideRootScale" null null))

(fn `Update Mouse Aim`
  (if (`self.Is Mouse Above Deadzone`)
    (`Controller.SetControlRotation` (`GameplayStatics.GetPlayerController` 0) (`self.Get Mouse Aim Direction`))))

(fn `Update Player Aim`
  (if (`self.Is Alive`)
    ;[1 0 0] TODO: Fix problem handle between control mobile and keyboard
    (if (`self.Gamepad Active`)
      (`self.Update Thumbstick Aim`)
      (else
        (`self.Update Mouse Aim`)))))

(fn `Update Thumbstick Aim`
  (if (`self.Is Thumbstick Above Deadzone`)
    (`Controller.SetControlRotation` (`GameplayStatics.GetPlayerController` 0) (`self.Get Thumbstick Aim Direction`))))

(fn `UserConstructionScript`)